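; Game mode for a shooter that tracks score and lives, starts enemy spawning and handles player respawn.
; On BeginPlay, a looping timer calls SpawnEnemy by name on the first EnemySpawn actor, at the EnemyPerSecond rate.
; RespawnPlayer destroys all enemies and deducts a life, then spawns and possesses a new hero.
; When lives reach zero, it shows the DeadUI with UI-only input instead.
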(event `IncrementScore`
  (params (DeltaScore :type Integer))
  ;[0.5089 0 1] Score
  (set `self.Score` (+ DeltaScore (`self.Score`))))

(event `self.ReceiveBeginPlay`
  ;[0.6947 1 0.2898] Spawn Enemys
  (bind _outactors (`GameplayStatics.GetAllActorsOfClass` "/Game/BluePrints/EnemySpawn.EnemySpawn_C"))
  (bind _output_get (set `self.EnemySpawner` (`|GetArrayItem` _outactors)))
  (`KismetSystemLibrary.K2_SetTimer` _output_get "SpawnEnemy" (/ 1.0 (`self.EnemyPerSecond`)) true))

(event `RespawnPlayer`
  (bind _returnvalue (`GameplayStatics.GetPlayerController` 0))
  ;[1 0 0.005858] Reset player after 3 dead show dead hud
  (bind _outactors (`GameplayStatics.GetAllActorsOfClass` "/Game/BluePrints/EnemyCharacter.EnemyCharacter_C"))
  (for _array_element _outactors
    (`self.K2_DestroyActor` _array_element))
  (set `self.life` (- (`self.life`) 1))
  (if (== (`self.life`) 0)
    (`self.DisableInput` (`GameplayStatics.GetPlayerController` 0))
    (`WidgetLayoutLibrary.RemoveAllWidgets`)
    (bind _returnvalue_2 (`|CreateWidget` "/Game/BluePrints/UI/DeadUI.DeadUI_C"))
    (`UserWidget.AddToViewport` _returnvalue_2 0)
    (set `PlayerController.bShowMouseCursor` true _returnvalue)
    (`WidgetBlueprintLibrary.SetInputMode_UIOnlyEx` _returnvalue _returnvalue_2)
    (else
      (bind _returnvalue_3 (`|SpawnActorFromClass` "/Game/BluePrints/HeroCharacter.HeroCharacter_C" (`self.PlayerSpawnTransform`) "Undefined" "MultiplyWithRoot" null null))
      (`Controller.Possess` (`GameplayStatics.GetPlayerController` 0) _returnvalue_3))))

(fn `UserConstructionScript`)