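; HeroCharacter is the player character for a shooter with twin-stick style controls, moving along world axes.
; On BeginPlay it spawns a weapon on the GunHold socket, records its spawn transform in ShooterMode and adds the ShooterHud.
; Both look axes share logic that sets control rotation and pulls the weapon trigger past a deadzone.
; AffecHealth updates health and, on death, disables input, then after a delay requests respawn and destroys weapon and character.
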(event `self.ReceiveBeginPlay`
  (bind _mesh (`self.Mesh`))
  (`|ExecutionSequence`
    (:`then_0`
      (bind _returnvalue (`|SpawnActorFromClass` "/Game/BluePrints/Weapon.Weapon_C" (`SceneComponent.K2_GetComponentToWorld` _mesh) "Undefined" "MultiplyWithRoot" null null))
      (bind _output_get (set `self.Weapon` _returnvalue))
      (`self.K2_AttachToComponent` _output_get _mesh "GunHold" "SnapToTarget" "KeepWorld" "KeepWorld" true))
    (:`then_1`
      (bind _asshooter_mode (cast `/Game/BluePrints/ShooterMode` (`GameplayStatics.GetGameMode`)))
      (bind _output_get_2 (set `self.GameMode` _asshooter_mode))
      (set `/Game/BluePrints/ShooterMode.PlayerSpawnTransform` (`self.GetTransform`) _output_get_2))
    (:`then_2`
      (bind _returnvalue_2 (`|GenericCreateObject` "/Game/BluePrints/UI/ShooterHud.ShooterHud_C"))
      (`UserWidget.AddToViewport` _returnvalue_2 0))))

(event `InputAxis|LookUp`
  (params (AxisValue :type "Float (single-precision)"))
  (bind _weapon (`self.Weapon`))
  ;[1 0.04418 0] Rotation
  (bind _returnvalue (`KismetMathLibrary.MakeVector` AxisValue (stale `InputAxis|LookRight` AxisValue)))
  (if (> (`KismetMathLibrary.VSize` _returnvalue) 0.25) :!label _label
    (`Controller.SetControlRotation` (`self.GetController`) (`KismetMathLibrary.Conv_VectorToRotator` _returnvalue))
    (`/Game/BluePrints/Weapon.PullTrigger` _weapon)
    (else
      (`/Game/BluePrints/Weapon.ReleaseTrigger` _weapon))))

(event `InputAxis|MoveUp`
  (params (AxisValue :type "Float (single-precision)"))
  ;[1 1 1] Movement
  (`self.AddMovementInput` (1.0 0.0 0.0) AxisValue))

(event `InputAxis|MoveRight`
  (params (AxisValue :type "Float (single-precision)"))
  ;[1 1 1] Movement
  (`self.AddMovementInput` (0.0 1.0 0.0) AxisValue))

(event `InputAxis|LookRight`
  (params (AxisValue :type "Float (single-precision)"))
  ;[1 0.04418 0] Rotation
  (goto _label))

(event `/Game/BluePrints/iDamageable.AffecHealth`
  (params (Delta :type "Float (double-precision)"))
  (`self.CalculateHealth` Delta)
  (if (`self.isDead`)
    (`self.DisableInput` (`GameplayStatics.GetPlayerController` 0))
    (`KismetSystemLibrary.Delay` 3.0)
    (`/Game/BluePrints/ShooterMode.RespawnPlayer` (`self.GameMode`))
    (`self.K2_DestroyActor` (`self.Weapon`))
    (`self.K2_DestroyActor` self)))

(fn `UserConstructionScript`)