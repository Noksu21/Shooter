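; Enemy character that deals repeated damage to an overlapping hero and awards score when killed.
; Overlap starts a looping timer that damages the hero at the attack rate, cleared when that hero leaves.
; AffecHealth calls CalculateHealth; on death it relaxes capsule collision, increments ShooterMode's score, detaches the controller, then explodes and destroys itself after a delay.
; The construction script tints the mesh through a dynamic material using EnemyColor.
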(event `/Game/BluePrints/iDamageable.AffecHealth`
  (params (Delta :type "Float (double-precision)"))
  (bind _capsulecomponent (`self.CapsuleComponent`))
  (`self.CalculateHealth` Delta)
  (if (`self.isDead`)
    (`PrimitiveComponent.SetCollisionResponseToChannel` _capsulecomponent "ECC_WorldDynamic" "ECR_Ignore")
    (`PrimitiveComponent.SetCollisionResponseToChannel` _capsulecomponent "ECC_Pawn" "ECR_Ignore")
    (bind _asshooter_mode (cast `/Game/BluePrints/ShooterMode` (`GameplayStatics.GetGameMode`)))
    (`/Game/BluePrints/ShooterMode.IncrementScore` _asshooter_mode (`self.Score`))
    (`self.DetachFromControllerPendingDestroy`)
    (`KismetSystemLibrary.Delay` 3.0)
    (`|SpawnActorFromClass` "/Game/BluePrints/Explosion.Explosion_C" (`self.GetTransform`) "Undefined" "MultiplyWithRoot" null null)
    (`self.K2_DestroyActor`)))

(event `self.ReceiveActorBeginOverlap`
  (params (OtherActor :type "Actor Object Reference"))
  (bind _ashero_character (cast `/Game/BluePrints/HeroCharacter` OtherActor))
  (set `self.Hero` _ashero_character)
  (`KismetSystemLibrary.K2_SetTimer` null "DamageToHero" (/ 1.0 (`self.AttacksPerSecond`)) true))

(event `DamageToHero`
  (`/Game/BluePrints/HeroCharacter.AffecHealth` (`self.Hero`) (`self.Damage`)))

(event `self.ReceiveActorEndOverlap`
  (params (OtherActor :type "Actor Object Reference"))
  (if (== OtherActor (`self.Hero`))
    (`KismetSystemLibrary.K2_ClearTimer` null "DamageToHero")))

(fn `UserConstructionScript`
  (bind _returnvalue (`PrimitiveComponent.CreateDynamicMaterialInstance` (`self.Mesh`) 0 null "None"))
  (bind _output_get (set `self.DynaMat` _returnvalue))
  (`MaterialInstanceDynamic.SetVectorParameterValue` _output_get "BodyColor" (`self.EnemyColor`)))